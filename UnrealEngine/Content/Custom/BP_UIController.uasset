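; UI controller for a flight display with detect-and-avoid threat bands around intruder aircraft.
; It creates and toggles the active WBP_UIDesign_19 widget and spawns BP_IntruderController from an intruder table.
; UpdateUI refreshes intruders, then passes ownship and closest-intruder positions to MyActor's FindIntersectionWithCircle, whose band feeds the widget.
; RasDaa also runs on Cesium-converted feet positions, but its result reaches only disconnected CSV logging; FakeDAIDALUS is an uncalled stub.
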(fn `AddIntruderData`
  (params (IntruderTable :type "DataTable Object Reference"))
  (bind _returnvalue (`|SpawnActorFromClass` "/Game/Custom/BP_IntruderController.BP_IntruderController_C" (`KismetMathLibrary.MakeTransform` (0.0 0.0 0.0)) "Undefined" "MultiplyWithRoot" null null))
  (bind _output_get (set `self.IntruderController` _returnvalue))
  (`/Game/Custom/BP_IntruderController.Activate` _output_get IntruderTable))

(fn `FakeDAIDALUS`
  (params (IntruderHeading :type "Float (double-precision)") (IntruderDistance :type "Float (double-precision)"))
  (returns (StartAngle :type "Float (double-precision)") (EndAngle :type "Float (double-precision)") (ThreatLevel :type Integer))
  (return (- IntruderHeading 25.0) (+ IntruderHeading 25.0) 2))

(fn `SetUI`
  (params (Selection :type Integer))
  (if (`KismetSystemLibrary.IsValid` (`self.ActiveUIObject`))
    (`/Game/Custom/BP_UI_Interface.Disable` (`self.ActiveUI`)))
  (switch `int` Selection
    (:`0`
      (bind _returnvalue (`|CreateWidget` "/Game/Custom/WBP_UIDesign_19.WBP_UIDesign_19_C" (`GameplayStatics.GetPlayerController` 0)))
      (set `self.ActiveUI` _returnvalue)
      (`UserWidget.AddToViewport` _returnvalue 0)
      (set `self.ActiveUIObject` _returnvalue)
      (`/Game/Custom/BP_UI_Interface.Initialize` _returnvalue)
      (set `Widget.Visibility` "Hidden" _returnvalue))
    (:`1`
      (bind _returnvalue_2 (`|CreateWidget` "/Game/Custom/WBP_UIDesign_19.WBP_UIDesign_19_C"))
      (set `self.ActiveUI` _returnvalue_2)
      (`UserWidget.AddToViewport` _returnvalue_2 0)
      (set `self.ActiveUIObject` _returnvalue_2)
      (`/Game/Custom/BP_UI_Interface.Initialize` _returnvalue_2)
      (set `Widget.Visibility` "Hidden" _returnvalue_2))))

(fn `ToggleUI`
  (bind _activeuiobject (`self.ActiveUIObject`))
  (if (`KismetSystemLibrary.IsValid` (`self.ActiveUIObject`))
    (if (`Widget.IsVisible` _activeuiobject)
      (`Widget.SetVisibility` _activeuiobject "Hidden")
      (else
        (`Widget.SetVisibility` _activeuiobject "Visible")))))

(fn `UpdateIntruder`
  (params (TopLeftCoords :type "Vector Structure") (TopRightCoords :type "Vector Structure") (BottomRightCoords :type "Vector Structure") (OwnshipAltitude :type "Float (double-precision)") (UseLast :type Boolean))
  (bind _intrudercontroller (`self.IntruderController`))
  (if (`KismetSystemLibrary.IsValid` _intrudercontroller)
    (`/Game/Custom/BP_IntruderController.Update` _intrudercontroller TopLeftCoords TopRightCoords BottomRightCoords OwnshipAltitude UseLast)))

(fn `UpdateUI`
  (params (OwnshipHeading :type "Float (double-precision)" :default -99999.0) (OwnshipLat :type "Float (double-precision)") (OwnshipLong :type "Float (double-precision)") (OwnshipAltitude :type "Float (double-precision)" :default -99999.0) (OwnshipGroundSpeed :type "Float (double-precision)" :default -99999.0) (OwnshipRoll :type "Float (double-precision)" :default -99999.0) (OwnshipPitch :type "Float (double-precision)" :default -99999.0) (FlightTime :type "Float (double-precision)" :default -99999.0) (Intruders :type "Array of /Game/Custom/BP_Intruder Object Reference") (TopLeftCoord :type "Vector Structure") (TopRightCoord :type "Vector Structure") (BottomRightCoord :type "Vector Structure") (BottomLeftCoord :type "Vector Structure") (Debug :type Boolean) (UseLast :type Boolean))
  (bind _returnvalue (`KismetMathLibrary.MakeVector` OwnshipLong OwnshipLat OwnshipAltitude))
  (if (`KismetSystemLibrary.IsValid` (`self.ActiveUIObject`))
    (if (`KismetSystemLibrary.IsValid` (`self.IntruderController`))
      (if (not UseLast)
        (`self.UpdateIntruder` TopLeftCoord TopRightCoord BottomRightCoord OwnshipAltitude)
        ;[1 1 1] DAIDULUS
        (bind _returnvalue_2 (`GameplayStatics.GetActorOfClass` "/Script/CesiumRuntime.CesiumGeoreference"))
        (if (> OwnshipHeading 180.0)
          (set `self.Ownship heading Var` (- OwnshipHeading 360.0))
          (else
            (set `self.Ownship heading Var` OwnshipHeading)))
        (bind (_intruderheading _intruderdistance _foundintruder _intruderloc) (`/Game/Custom/BP_IntruderController.GetClosestIntruderData` (`self.IntruderController`) _returnvalue)) ; Gets closest intruder and returns its heading and distance for now -- later will return relevant data for daidalus
        (if (> _intruderheading 180.0)
          (set `self.Intruder heading Var` (- _intruderheading 360.0))
          (else
            (set `self.Intruder heading Var` _intruderheading)))
        (bind _returnvalue_3 (`GameplayStatics.GetActorOfClass` "/Script/CesiumRuntime.CesiumGeoreference"))
        ;[1 1 1] New DAA
        (bind _returnvalue_4 (`GameplayStatics.GetActorOfClass` "/Script/UEReferenceApp.MyActor"))
        (bind _structout (setmembers `Aircraft` :`StructRef` (make `Aircraft` -50.0) :`x` OwnshipLat :`y` OwnshipLong :`speed` 250.0 :`heading` 30.0 :`dir` (`|MakeArray` 0.0)))
        (bind _structout_2 (setmembers `Aircraft` :`StructRef` (make `Aircraft` -50.0 22.0) :`x` (.x _intruderloc) :`y` (.y _intruderloc) :`speed` 250.0 :`heading` 60.0 :`dir` (`|MakeArray` 0.0)))
        (bind _structout_3 (setmembers `NewParameters` :`StructRef` (make `NewParameters` 8000.0) :`art` 8000.0 :`sst` 12000.0))
        (bind (_startangle _endangle _level) (`MyActor.findIntersectionWithCircle` _returnvalue_4 _structout_3 _structout _structout_2))
        (`KismetSystemLibrary.PrintString` (`KismetStringLibrary.Conv_VectorToString` (`KismetMathLibrary.MakeVector` _startangle _endangle (`KismetMathLibrary.Conv_IntToDouble` _level))))
        (bind (_startangle_2 _endangle_2 _alert) (`MyActor.RasDaa` _returnvalue_4 (`KismetMathLibrary.MakeVector` (.y (* (`CesiumGeoreference.TransformLongitudeLatitudeHeightPositionToUnreal` _returnvalue_2 _returnvalue) (0.032808 0.032808 0.032808))) (.x (* (`CesiumGeoreference.TransformLongitudeLatitudeHeightPositionToUnreal` _returnvalue_2 _returnvalue) (0.032808 0.032808 0.032808))) (.z (* (`CesiumGeoreference.TransformLongitudeLatitudeHeightPositionToUnreal` _returnvalue_2 _returnvalue) (0.032808 0.032808 0.032808)))) (`KismetMathLibrary.MakeVector` (.y (* (`CesiumGeoreference.TransformLongitudeLatitudeHeightPositionToUnreal` _returnvalue_3 _intruderloc) (0.032808 0.032808 0.032808))) (.x (* (`CesiumGeoreference.TransformLongitudeLatitudeHeightPositionToUnreal` _returnvalue_3 _intruderloc) (0.032808 0.032808 0.032808))) (.z (* (`CesiumGeoreference.TransformLongitudeLatitudeHeightPositionToUnreal` _returnvalue_3 _intruderloc) (0.032808 0.032808 0.032808)))) (`KismetMathLibrary.MakeVector` (`self.Ownship heading Var`) OwnshipGroundSpeed) (`KismetMathLibrary.MakeVector` (`self.Intruder heading Var`) (`self.Intruder Speed Var`)) (make `Parameters` 2000.0)))
        (`/Game/Custom/BP_UI_Interface.UpdateUI` (`self.ActiveUI`) OwnshipHeading OwnshipAltitude OwnshipGroundSpeed OwnshipRoll OwnshipPitch FlightTime _startangle _endangle _level Intruders TopLeftCoord TopRightCoord BottomRightCoord BottomLeftCoord Debug :!label _label)
        (else
          (`self.UpdateIntruder` TopLeftCoord TopRightCoord BottomRightCoord OwnshipAltitude true)))
      (else
        (goto _label)))))

(fn `UserConstructionScript`)